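; A flower actor that grows in small random steps after it spawns.
; On BeginPlay it runs three rounds, each waiting a random few seconds and then enlarging the Plane001 mesh by a small random amount.
; Each step adds the increment to the current world scale and writes the result as relative scale, so growth stops after the third step.
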(event `self.ReceiveBeginPlay`
  (bind _returnvalue (`KismetMathLibrary.RandomFloatInRange` 3.0 8.0))
  (bind _returnvalue_2 (`KismetMathLibrary.RandomFloatInRange` 0.02 0.1))
  (bind _plane_001 (`self.Plane_001`))
  (bind _plane_001_2 (`self.Plane_001`))
  (bind _plane_001_3 (`self.Plane_001`))
  (`KismetSystemLibrary.Delay` _returnvalue)
  (`SceneComponent.SetRelativeScale3D` _plane_001_2 (+ (`SceneComponent.K2_GetComponentScale` _plane_001_2) _returnvalue_2))
  (`KismetSystemLibrary.Delay` _returnvalue)
  (`SceneComponent.SetRelativeScale3D` _plane_001_3 (+ (`SceneComponent.K2_GetComponentScale` _plane_001_3) _returnvalue_2))
  (`KismetSystemLibrary.Delay` _returnvalue)
  (`SceneComponent.SetRelativeScale3D` _plane_001 (+ (`SceneComponent.K2_GetComponentScale` _plane_001) _returnvalue_2)))

(fn `UserConstructionScript`)