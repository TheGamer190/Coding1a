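; BP_LoopsandLists is a demo actor exercising loops, arrays and debug text printing.
; After BeginPlay, one delayed branch runs a while loop that counts Counter down to zero, printing each value in a color cycled from the Colors array by modulo.
; The other starts MakeCoinsJump, which raises every BP_Key actor's root, prints how many moved, then calls itself after a delay, repeating indefinitely.
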(event `self.ReceiveBeginPlay`
  (bind _counter (`self.counter`))
  ; Print text in different colors
  (`|ExecutionSequence`
    (:`then_0`
      (`KismetSystemLibrary.Delay` 2.0)
      (while (> _counter 0)
        (`KismetSystemLibrary.PrintText` (`|FormatText` "Current counter in loop is {counter}" _counter) true true (`|GetArrayItem` (`self.colors`) (mod _counter 7)))
        (`/Engine/EditorBlueprintResources/StandardMacros.DecrementInt` _counter)))
    (:`then_1`
      (`KismetSystemLibrary.Delay` 0.2)
      (`self.MakeCoinsJump`))))

(event `MakeCoinsJump`
  ; Movecoins up
  (bind _outactors (`GameplayStatics.GetAllActorsOfClass` "/Game/Blueprints/BP_Key.BP_Key_C"))
  (for _array_element _outactors
    (`SceneComponent.K2_AddRelativeLocation` (`/Game/Blueprints/BP_Key.DefaultSceneRoot` _array_element) (0.0 0.0 50.0) false false))
  (`KismetSystemLibrary.PrintText` (`|FormatText` "We have raised {counter} keys!" (`KismetArrayLibrary.Array_Length` _outactors)))
  (`KismetSystemLibrary.Delay` 1.0)
  (`self.MakeCoinsJump`))

(fn `UserConstructionScript`)