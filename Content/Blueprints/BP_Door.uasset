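; BP_Door is a coin-gated door that spends one of the player's coins to open when a BP_ThirdPersonCharacter overlaps it.
; A timeline swings the door mesh through a 90-degree yaw, printing a message on success or refusal.
; The timeline's Update output also activates a Niagara effect and runs a two-second Delay, after which the door actor destroys itself.
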(event `self.ReceiveActorBeginOverlap`
  (params (OtherActor :type "Actor Object Reference"))
  (bind _asbp_third_person_character (cast `/Game/ThirdPerson/Blueprints/BP_ThirdPersonCharacter` OtherActor))
  (if (> (`/Game/ThirdPerson/Blueprints/BP_ThirdPersonCharacter.coinsCollected` _asbp_third_person_character) 0)
    (`/Engine/EditorBlueprintResources/StandardMacros.DecrementInt` (`/Game/ThirdPerson/Blueprints/BP_ThirdPersonCharacter.coinsCollected` _asbp_third_person_character)
      (:`  `
        (`KismetSystemLibrary.PrintText` "Door open")
        (bind (_direction _newtrack_0) (`Timeline|Swint door open`)
          (:`Update`
            (`SceneComponent.K2_SetRelativeRotation` (`self.SM_Bld_Door_01`) (`KismetMathLibrary.MakeRotator` 0.0 0.0 (`KismetMathLibrary.Lerp` 0.0 -90.0 _newtrack_0)) false false)
            (`ActorComponent.Activate` (`self.NewNiagaraSystem`) false)
            (`KismetSystemLibrary.Delay` 2.0)
            (`self.K2_DestroyActor`)))))
    (else
      (`KismetSystemLibrary.PrintText` "Door shall not open "))))

(fn `UserConstructionScript`)