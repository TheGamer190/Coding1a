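; BP_DialogueManager shows lines from a DialogueStrings array on the player's HUD, one per DisplayNextLine call.
; Each call wraps ArrayIndex to the start past the last entry, shows that line, then increments the index.
; ShowDialogue casts the player to BP_ThirdPersonCharacter, sets its widget's dialogue text, and clears it after a two-second delay.
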(event `DisplayNextLine`
  ; Check if the index isn't out of bounds, if so then print text the current diaglouge index
  (if (>= (`self.arrayIndex`) (`KismetArrayLibrary.Array_Length` (`self.dialogueStrings`)))
    (set `self.arrayIndex` 0))
  (`self.ShowDialogue`)
  (`/Engine/EditorBlueprintResources/StandardMacros.IncrementInt` (`self.arrayIndex`)))

(event `ShowDialogue`
  (bind _asbp_third_person_character (cast `/Game/ThirdPerson/Blueprints/BP_ThirdPersonCharacter` (`GameplayStatics.GetPlayerCharacter` 0)))
  (bind _dialogie (`/Game/UI/UI_TotalSeeds.Dialogie` (`/Game/ThirdPerson/Blueprints/BP_ThirdPersonCharacter.Widget` _asbp_third_person_character)))
  (`TextBlock.SetText` _dialogie (`|GetArrayItem` (`self.dialogueStrings`) (`self.arrayIndex`)))
  (`KismetSystemLibrary.Delay` 2.0)
  (`TextBlock.SetText` _dialogie ""))

(fn `UserConstructionScript`)