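; BP_Launcher is a cannon actor that fires one cannonball one second after play begins and another whenever an actor begins overlapping it, without delay.
; Each shot calls LaunchCanonBall, which only prints a message, then spawns a BP_CannonBall at the spawn point component.
; The ball's Cube is pushed along its own forward vector by ShootForce, applied as a mass-independent acceleration change.
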(event `Launch Canon Ball`
  (`KismetSystemLibrary.PrintText` "Ka pow!!"))

(event `self.ReceiveBeginPlay`
  (`KismetSystemLibrary.Delay` 1.0)
  (`self.Launch Canon Ball` :!label _label)
  (bind _returnvalue (`|SpawnActorFromClass` "/Game/Blueprints/BP_CannonBall.BP_CannonBall_C" (`SceneComponent.K2_GetComponentToWorld` (`self.SpanwPoint`)) "Undefined" "MultiplyWithRoot" null null))
  (bind _cube (`/Game/Blueprints/BP_CannonBall.Cube` _returnvalue))
  (`PrimitiveComponent.AddForce` _cube (* (`SceneComponent.GetForwardVector` _cube) (`self.shootForce`)) "None" true))

(event `self.ReceiveActorBeginOverlap`
  (params (OtherActor :type "Actor Object Reference"))
  (goto _label))

(fn `UserConstructionScript`)