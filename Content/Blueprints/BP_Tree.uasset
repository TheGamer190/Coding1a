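; BP_Tree is a tree Blueprint that grows in steps after play begins.
; BeginPlay runs a delay loop while GrowCounter is above zero, waiting a random few seconds, enlarging the StaticMesh by a random uniform amount and decrementing the counter.
; Each step reads the mesh's world scale and writes the result as relative scale.
; Leftover disconnected delay, scale and loop nodes never run.
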(event `self.ReceiveBeginPlay`
  (bind _staticmesh (`self.StaticMesh`))
  (if (> (`self.growCounter`) 0) :!label _label
    ; Comment
    (`KismetSystemLibrary.Delay` (`KismetMathLibrary.RandomFloatInRange` 3.0 8.0))
    (`SceneComponent.SetRelativeScale3D` _staticmesh (+ (`SceneComponent.K2_GetComponentScale` _staticmesh) (`KismetMathLibrary.RandomFloatInRange` 0.2 0.8)))
    (`/Engine/EditorBlueprintResources/StandardMacros.DecrementInt` (`self.growCounter`)
      (:`  `
        (goto _label)))))

(fn `UserConstructionScript`)